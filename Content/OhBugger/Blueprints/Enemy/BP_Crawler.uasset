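; BP_Crawler is an enemy Blueprint for a crawler that roams continuously from BeginPlay.
; OnRoam eases the root component toward random navmesh-derived XY points at a fixed height via MoveComponentTo, pauses, then calls itself again.
; AI Perception sets Target and an Attack or Idle state and prints updated actor names.
; Nothing live reads that state: the Idle-to-Roam switch is unwired, and no attack logic exists here.
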(event OnPerceptionUpdated(AIPerception)
  (params (UpdatedActors :type Array%20of%20Actor%20Object%20References))
  (for _array_element UpdatedActors
    (Development|PrintString (Utilities|GetDisplayName _array_element))))

(event OnTargetPerceptionUpdated(AIPerception)
  (params (Actor :type Actor%20Object%20Reference) (Stimulus :type AI%20Stimulus%20Structure))
  (if (.bSuccessfullySensed (Utilities|Struct|BreakAIStimulus Stimulus))
    (Variables|Default|SetTarget Actor)
    (Variables|Default|SetState "NewEnumerator2")
    (else
      (Variables|Default|SetTarget 0)
      (Variables|Default|SetState "NewEnumerator0"))))

(event Custom|OnRoam
  (bind _returnvalue (Transformation|GetActorLocation))
  (bind _randomlocation (AI|Navigation|GetRandomReachablePointinRadius _returnvalue 2.5e+03 0 0))
  (Components|MoveComponentTo (Variables|Default|GetDefaultSceneRoot) (Math|Vector|MakeVector (.x _randomlocation) (.y _randomlocation) 1e+02) "0, 0, 0" true true 5.0 false)
  (Utilities|FlowControl|Delay 2.0)
  (CallFunction|OnRoam))

(event EventBeginPlay
  (|CallParentFunction)
  (CallFunction|OnRoam))

(event Collision|EventActorBeginOverlap
  (params (OtherActor :type Actor%20Object%20Reference))
  (|CallParentFunction OtherActor) ; This node is disabled and will not be called.\nDrag off pins to build functionality.
)

(event EventTick
  (params (DeltaSeconds :type Float%20%28single-precision%29))
  (|CallParentFunction DeltaSeconds))

(fn ConstructionScript
  (|CallParentFunction))