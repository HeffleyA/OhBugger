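; BP_EnemyController is an AI controller that sends its enemy pawn to a random reachable point nearby.
; Shortly after possession, it calls MoveToRandomLocation once, which picks a navigable point within a fixed radius of the pawn.
; A separate MoveToRandom event does a similar AIMoveTo but is not called here.
; BeginPlay and Tick do no effective work, and a second delayed move is disconnected.
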(event Custom|MoveToRandom
  (bind _self self)
  (bind _returnvalue (Pawn|GetControlledPawn _self))
  (AI|AIMoveTo _returnvalue (.RandomLocation (AI|Navigation|GetRandomReachablePointinRadius (Transformation|GetActorLocation _returnvalue) 0.0 0 0)) 0 5.0 false))

(event EventBeginPlay
  (switch Utilities|FlowControl|Switch|SwitchonE_EnemyState "NewEnumerator0"))

(event EventTick
  (params (DeltaSeconds :type Float%20%28single-precision%29)))

(event EventPossess
  (params (PossessedPawn :type Pawn%20Object%20Reference))
  (Utilities|FlowControl|Delay 0.1)
  (CallFunction|MovetoRandomLocation))

(fn ConstructionScript)

(fn MovetoRandomLocation
  (AI|Navigation|MovetoLocation (.RandomLocation (AI|Navigation|GetRandomReachablePointinRadius (Transformation|GetActorLocation (Pawn|GetControlledPawn self)) 1e+03 0 0)) -1.0 true true false true 0))