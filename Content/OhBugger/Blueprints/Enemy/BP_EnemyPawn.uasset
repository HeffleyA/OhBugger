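; Enemy pawn that wanders by moving to a random reachable point within a fixed radius on a looping one-second timer.
; Tick smoothly rotates it toward its velocity.
; An unfinished boids-style Flocking function, never called here, steers toward perceived actors' average position and feeds FloatingPawnMovement acceleration.
; Separation and Alignment are empty, and ClampMagnitude returns zero for over-limit vectors.
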(event Custom|OnMove
  (AI|AIMoveTo self (.RandomLocation (AI|Navigation|GetRandomReachablePointinRadius (Transformation|GetActorLocation) 1e+03 0 0)) 0 5.0 false))

(event Custom|OnBeginMove
  (Utilities|Time|SetTimerbyEvent (delegate Custom|OnMove) 1.0 true))

(event EventBeginPlay
  (CallFunction|OnBeginMove))

(event Collision|EventActorBeginOverlap
  (params (OtherActor :type Actor%20Object%20Reference)))

(event EventTick
  (params (DeltaSeconds :type Float%20%28single-precision%29))
  (Transformation|SetActorRotation (Math|Interpolation|RInterpTo (Transformation|GetActorRotation) (Math|Rotator|MakeRotfromX (Transformation|GetVelocity)) DeltaSeconds 5.0)))

(fn ConstructionScript)

(fn Flocking
  (bind _aiperception (Variables|Default|GetAIPerception))
  (bind _floatingpawnmovement (Variables|Default|GetFloatingPawnMovement))
  (bind _outactors (Class|AIPerceptionComponent|GetCurrentlyPerceivedActors _aiperception))
  (if (> (Utilities|Array|Length _outactors) 0)
    (bind _force (CallFunction|Cohesion _outactors))
    (bind _newaccel (CallFunction|ApplyForce _force (Variables|/Script/Engine.FloatingPawnMovement|GetAcceleration _floatingpawnmovement)))
    (Variables|/Script/Engine.FloatingPawnMovement|SetAcceleration _floatingpawnmovement _newaccel)))

(fn Cohesion
  (params (Neighbors :type Array%20of%20Actor%20Object%20References))
  (for _array_element Neighbors
    (LocalVariables|SetPositions (+ (LocalVariables|GetPositions) (Transformation|GetActorLocation _array_element))))
  (bind _force (CallFunction|GetSteeringForce (- (/ (LocalVariables|GetPositions) (Utilities|Array|Length Neighbors)) (Transformation|GetActorLocation))))
  (return _force))

(fn Separation
  (params (Neighbors :type Array%20of%20Actor%20Object%20References) (Radius :type Float%20%28double-precision%29)))

(fn Alignment)

(fn GetSteeringForce
  (params (Direction :type Vector))
  (bind _floatingpawnmovement (Variables|Default|GetFloatingPawnMovement))
  (bind _vectorout (CallFunction|ClampMagnitude (- (* (Class|MovementComponent|GetMaxSpeed _floatingpawnmovement) (Math|Vector|Normalize Direction)) (Variables|/Script/Engine.MovementComponent|GetVelocity _floatingpawnmovement)) 5.0))
  (return _vectorout))

(fn ClampMagnitude
  (params (Vector :type Vector) (MaxLength :type Float%20%28double-precision%29))
  (bind _returnvalue (Math|Vector|VectorLength Vector))
  (if (> _returnvalue MaxLength)
    (return (Math|Vector|MakeVector (* (/ 0.0 _returnvalue) MaxLength) (* (/ 0.0 _returnvalue) MaxLength) (* (/ 0.0 _returnvalue) MaxLength)))
    (else
      (return Vector))))

(fn ApplyForce
  (params (Force :type Vector) (Acceleration :type Float%20%28double-precision%29))
  (return (Math|Vector|VectorLength (+ Force (Math|Vector|MakeVector Acceleration Acceleration Acceleration)))))