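; BP_EnemySpawner is a roaming spawner that releases ever-larger swarms of BP_EnemyPawn enemies.
; A Tick countdown triggers a swarm, then resets to a minute.
; Each swarm first teleports the spawner to a random navigable point near its current location, then loops AI spawns at that single spot.
; SwarmSize doubles after every wave, so enemy counts grow exponentially with no cap.
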(event Custom|OnSwarm
  (bind _randomlocation (Class|NavigationSystemV1|GetRandomLocationinNavigableRadius (Transformation|GetActorLocation) 1e+03 0 0))
  (Transformation|SetActorLocation _randomlocation false true)
  (for _index (range 0 (Variables|Default|GetSwarmSize))
    (CallFunction|OnSpawnEnemy))
  (Variables|Default|SetSwarmSize (* (Variables|Default|GetSwarmSize) 2)))

(event Custom|OnSpawnEnemy
  (AI|SpawnAIFromClass "/Game/OhBugger/Blueprints/Enemy/BP_EnemyPawn.BP_EnemyPawn_C" 0 (Transformation|GetActorLocation) "0, 0, 0" false 0))

(event EventBeginPlay)

(event Collision|EventActorBeginOverlap
  (params (OtherActor :type Actor%20Object%20Reference)))

(event EventTick
  (params (DeltaSeconds :type Float%20%28single-precision%29))
  (if (<= (Variables|Default|GetTimer) 0.0)
    (CallFunction|OnSwarm)
    (Variables|Default|SetTimer 6e+01)
    (else
      (Variables|Default|SetTimer (- (Variables|Default|GetTimer) DeltaSeconds)))))

(fn ConstructionScript)