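; BP_PickupSpawner is an actor that periodically spawns health or ammo pickups at random reachable spots in the level.
; Tick counts down a timer and fires OnSpawnPickup every five seconds.
; That event teleports the spawner to a random navmesh point within a large radius of its current location, then spawns one of the two pickups there with equal odds.
; Because the spawner itself moves, each search starts from the previous spawn point.
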(event Custom|OnSpawnPickup
  (bind _randomlocation (Class|NavigationSystemV1|GetRandomLocationinNavigableRadius (Transformation|GetActorLocation) 5e+03 0 0))
  (Transformation|SetActorLocation _randomlocation false true)
  (if (== (Math|Random|RandomInteger 2) 0)
    (Game|SpawnActorfromClass "/Game/OhBugger/Blueprints/Pickups/BP_HealthPickup.BP_HealthPickup_C" (Math|Transform|MakeTransform (Transformation|GetActorLocation) "0, 0, 0" "1.000000,1.000000,1.000000") "Undefined" "MultiplyWithRoot" 0 0)
    (else
      (Game|SpawnActorfromClass "/Game/OhBugger/Blueprints/Pickups/BP_AmmoPickup.BP_AmmoPickup_C" (Math|Transform|MakeTransform (Transformation|GetActorLocation) "0, 0, 0" "1.000000,1.000000,1.000000") "Undefined" "MultiplyWithRoot" 0 0))))

(event EventBeginPlay)

(event Collision|EventActorBeginOverlap
  (params (OtherActor :type Actor%20Object%20Reference)))

(event EventTick
  (params (DeltaSeconds :type Float%20%28single-precision%29))
  (if (<= (Variables|Default|GetTimer) 0.0)
    (CallFunction|OnSpawnPickup)
    (Variables|Default|SetTimer 5.0)
    (else
      (Variables|Default|SetTimer (- (Variables|Default|GetTimer) DeltaSeconds)))))

(fn ConstructionScript)