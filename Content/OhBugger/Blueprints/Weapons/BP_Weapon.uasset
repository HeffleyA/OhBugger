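; BP_Weapon is a weapon actor that fires projectiles according to the fire type in its WeaponData struct.
; OnStartFire fires once for Single, starts a looping FireRate timer for Automatic, or zeroes rate and ammo for None.
; OnFire spawns the projectile at the mesh's named socket and decrements ammo.
; The graph contains no ammo check or logic to stop the timer.
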(event Custom|OnFire
  (Game|SpawnActorfromClass (.projectile (Variables|Default|GetWeaponData)) (Transformation|GetSocketTransform (Variables|Default|GetStaticMesh) (.socket (Variables|Default|GetWeaponData)) "RTS_World") "Undefined" "MultiplyWithRoot" 0 0)
  (Variables|Default|SetWeaponData (Utilities|Struct|MakeS_WeaponData (.name (Variables|Default|GetWeaponData)) (.firetype (Variables|Default|GetWeaponData)) (.firerate (Variables|Default|GetWeaponData)) (.mesh (Variables|Default|GetWeaponData)) (.socket (Variables|Default|GetWeaponData)) (.projectile (Variables|Default|GetWeaponData)) (.weapon (Variables|Default|GetWeaponData)) (- (.ammo (Variables|Default|GetWeaponData)) 1.0))))

(event Custom|OnStartFire
  (switch Utilities|FlowControl|Switch|SwitchonE_FireType (.firetype (Variables|Default|GetWeaponData))
    (:NewEnumerator2
      (Variables|Default|SetWeaponData (Utilities|Struct|MakeS_WeaponData (.name (Variables|Default|GetWeaponData)) "NewEnumerator2" 0.0 (.mesh (Variables|Default|GetWeaponData)) (.socket (Variables|Default|GetWeaponData)) (.projectile (Variables|Default|GetWeaponData)) (.weapon (Variables|Default|GetWeaponData)) 0.0)))
    (:NewEnumerator0
      (CallFunction|OnFire))
    (:NewEnumerator1
      (Utilities|Time|SetTimerbyEvent (delegate Custom|OnFire) (.firerate (Variables|Default|GetWeaponData)) true))))

(event EventBeginPlay)

(event Collision|EventActorBeginOverlap
  (params (OtherActor :type Actor%20Object%20Reference)))

(event EventTick
  (params (DeltaSeconds :type Float%20%28single-precision%29)))

(fn ConstructionScript)