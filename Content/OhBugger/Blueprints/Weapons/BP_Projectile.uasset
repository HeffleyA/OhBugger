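; BP_Projectile is a weapon projectile that damages the first actor it overlaps and then destroys itself.
; The construction script sets the ProjectileMovement initial speed and a starting Lifespan value.
; Tick counts Lifespan down manually and destroys the projectile when it runs out.
; The overlap handler applies fixed damage without filtering which actor it touches.
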(event EventBeginPlay)

(event Collision|EventActorBeginOverlap
  (params (OtherActor :type Actor%20Object%20Reference))
  (Game|Damage|ApplyDamage OtherActor 1e+01 0 0)
  (Actor|DestroyActor))

(event EventTick
  (params (DeltaSeconds :type Float%20%28single-precision%29))
  (bind _output_get (Variables|Default|SetLifespan (- (Variables|Default|GetLifespan) DeltaSeconds)))
  (if (<= _output_get 0.0)
    (Actor|DestroyActor)))

(fn ConstructionScript
  (Variables|/Script/Engine.ProjectileMovementComponent|SetInitialSpeed (Variables|Default|GetProjectileMovement) 1e+03)
  (Variables|Default|SetLifespan 1e+01))